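; Front-end player controller that hosts the menu UI.
; On BeginPlay it creates and activates the WBP_UIBase root widget, switches to UI-only input with a visible, locked cursor, then loads and applies the saved game user settings.
; Pass-through events forward penta and flyout menu pushes, title updates and menu enable/disable to that root widget.
; These forwarders are noted as possibly removable, since "Find Parent of Class" now exists.
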(event `self.ReceiveBeginPlay`
  ;[1 1 1] Initialization
  (bind _returnvalue (`|CreateWidget` "/Game/Blueprints/UI/WBP_UIBase.WBP_UIBase_C" self))
  (bind _output_get (set `self.UIBase` _returnvalue))
  (`UserWidget.AddToViewport` _output_get 0)
  (`CommonActivatableWidget.ActivateWidget` (`self.UIBase`))
  (`WidgetBlueprintLibrary.SetInputMode_UIOnlyEx` self (`self.UIBase`) "LockAlways")
  (set `self.bShowMouseCursor` true)
  (bind _returnvalue_2 (`GameUserSettings.GetGameUserSettings`))
  (`GameUserSettings.LoadSettings` _returnvalue_2 false)
  (`GameUserSettings.ApplySettings` _returnvalue_2 true))

(event `/Game/Blueprints/UI/BPI_UIMain.PushPentaMenu`
  (params (`Widget Class` :type "CommonActivatableWidget Class Reference"))
  ;[1 1 1] We can probably remove these at some point since we have "Find Parent of Class" now
  (`/Game/Blueprints/UI/BPI_UIMain.PushPentaMenu` (`self.UIBase`) `Widget Class`))

(event `/Game/Blueprints/UI/BPI_UIMain.PushFlyoutMenu`
  (params (`Widget Class` :type "CommonActivatableWidget Class Reference") (`Flyout Position` :type "/Game/E_FlyoutMenus Enum" :default "NewEnumerator0"))
  ;[1 1 1] We can probably remove these at some point since we have "Find Parent of Class" now
  (`/Game/Blueprints/UI/WBP_UIBase.PushFlyoutMenu` (`self.UIBase`) `Widget Class` `Flyout Position`))

(event `/Game/Blueprints/UI/BPI_UIMain.UpdateMenuTitle`
  (params (Title :type Text))
  ;[1 1 1] We can probably remove these at some point since we have "Find Parent of Class" now
  (`/Game/Blueprints/UI/WBP_UIBase.UpdateMenuTitle` (`self.UIBase`) Title))

(event `/Game/Blueprints/UI/BPI_UIMain.DisableMenu`
  (`/Game/Blueprints/UI/WBP_UIBase.DisableMenu` (`self.UIBase`)))

(event `/Game/Blueprints/UI/BPI_UIMain.EnableMenu`
  (`/Game/Blueprints/UI/WBP_UIBase.EnableMenu` (`self.UIBase`)))

(fn `UserConstructionScript`)